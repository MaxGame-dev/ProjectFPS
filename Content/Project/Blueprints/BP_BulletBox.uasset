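; BP_BulletBox is an ammo pickup that gives bullets to the first-person character on overlap.
; The Box overlap casts to BP_FirstPersonCharacter, calls UpdateOwnBullet and plays a sound at the box's location.
; UpdateActive flips the Active flag, switching STMBox visibility and Box query collision together.
; It runs on pickup and again after a fixed delay, so the box respawns in place without being destroyed.
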(event `self.Box.OnComponentBeginOverlap`
  (params (OverlappedComponent :type "PrimitiveComponent Object Reference") (OtherActor :type "Actor Object Reference") (OtherComp :type "PrimitiveComponent Object Reference") (OtherBodyIndex :type Integer) (bFromSweep :type Boolean) (SweepResult :type "HitResult Structure (by ref)"))
  (bind _asbp_first_person_character (cast `/Game/FirstPerson/Blueprints/BP_FirstPersonCharacter` OtherActor))
  (`/Game/FirstPerson/Blueprints/BP_FirstPersonCharacter.UpdateOwnBullet` _asbp_first_person_character 5)
  (`GameplayStatics.PlaySoundAtLocation` "/Game/Game_Item/Pick_Up/Wav/Wav_Ashorttactilesou3_wav.Wav_Ashorttactilesou3_wav" (`self.K2_GetActorLocation`) (struct) 1.0 1.0 0.0 null null null null)
  (`self.UpdateActive`)
  (`KismetSystemLibrary.Delay` 10.0)
  (`self.UpdateActive`))

(event `UpdateActive`
  (bind _output_get (set `self.bActive` (not (`self.bActive`))))
  (`SceneComponent.SetVisibility` (`self.STM_Box`) _output_get false)
  (if _output_get
    (`PrimitiveComponent.SetCollisionEnabled` (`self.Box`) "QueryOnly")
    (else
      (`PrimitiveComponent.SetCollisionEnabled` (`self.Box`) "NoCollision"))))

(fn `UserConstructionScript`)